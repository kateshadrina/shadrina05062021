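; Explosive barrel that loses health when AmmoBase actors overlap it, then catches fire and explodes at low health.
; After a short fuse it plays the blast sound, briefly expands two damage spheres, fires a radial impulse and removes itself.
; The character sphere damages or kills MainCharacter through HealthStats.
; Any overlap on the barrel sphere cuts health and starts detonation without a threshold check, allowing chain reactions.
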(event OnComponentBeginOverlap(Capsule)
  (params (OverlappedComponent :type Primitive%20Component%20Object%20Reference) (OtherActor :type Actor%20Object%20Reference) (OtherComp :type Primitive%20Component%20Object%20Reference) (OtherBodyIndex :type Integer) (bFromSweep :type Boolean) (SweepResult :type Hit%20Result%20Structure%20%28by%20ref%29)))

(event OnComponentBeginOverlap(Char_Damage)
  (params (OverlappedComponent :type Primitive%20Component%20Object%20Reference) (OtherActor :type Actor%20Object%20Reference) (OtherComp :type Primitive%20Component%20Object%20Reference) (OtherBodyIndex :type Integer) (bFromSweep :type Boolean) (SweepResult :type Hit%20Result%20Structure%20%28by%20ref%29))
  (bind _asmain_character (Utilities|Casting|CastToMainCharacter OtherActor))
  (if (> (Variables|/Game/kateshadrina/Characters/MainCharacter.MainCharacter_C|GetHealth _asmain_character) 0)
    (Default|DoDamage (Variables|/Game/kateshadrina/Characters/MainCharacter.MainCharacter_C|GetHealthStats _asmain_character) 3e+01)
    (if (<= (Variables|/Game/kateshadrina/Characters/MainCharacter.MainCharacter_C|GetHealth _asmain_character) 0)
      (Default|Death (Variables|/Game/kateshadrina/Characters/MainCharacter.MainCharacter_C|GetHealthStats _asmain_character))
      (Audio|SpawnSoundatLocation "/Game/kateshadrina/Audio/DamageAndDeath/death.death" "0, 0, 0" "0, 0, 0" 1.0 1.0 0.0 0 0))))

(event OnComponentBeginOverlap(barrel_damage)
  (params (OverlappedComponent :type Primitive%20Component%20Object%20Reference) (OtherActor :type Actor%20Object%20Reference) (OtherComp :type Primitive%20Component%20Object%20Reference) (OtherBodyIndex :type Integer) (bFromSweep :type Boolean) (SweepResult :type Hit%20Result%20Structure%20%28by%20ref%29))
  (bind _teraccgda (Variables|Default|Getteraccgda))
  (bind _char_damage (Variables|Default|GetChar_Damage))
  (Variables|Default|Setbarrel_health (- (Variables|Default|Getbarrel_health) 8e+01))
  (Rendering|SetVisibility (Variables|Default|GetPointLight) true false)
  (Components|Activation|Activate (Variables|Default|Getfire) false)
  (Utilities|FlowControl|Delay 2.0)
  (Audio|PlaySound2D "/Game/StarterContent/Audio/Explosion_Cue.Explosion_Cue" 1.0 1.0 0.0 0 0)
  (Utilities|IsValid _char_damage
    (:Is%20Valid
      (Components|Sphere|SetSphereRadius _char_damage 1e+03 true)
      (Components|Sphere|SetSphereRadius (Variables|Default|Getbarrel_damage) 1e+03 true)
      (Components|DestroyComponent _char_damage))
    (:Is%20Not%20Valid
      _))
  (Class|RadialForceComponent|FireImpulse (Variables|Default|GetRadialForce))
  (Components|Activation|SetAutoActivate (Variables|Default|Getexp) false)
  (Utilities|IsValid _teraccgda
    (:Is%20Valid
      (Components|DestroyComponent _teraccgda)
      (Utilities|FlowControl|Delay 0.2)
      (Components|Activation|Deactivate (Variables|Default|Getfire))
      (Rendering|SetVisibility (Variables|Default|GetPointLight) false false)
      (Utilities|FlowControl|Delay 1.0)
      (Actor|DestroyActor))))

(event EventBeginPlay)

(event Collision|EventActorBeginOverlap
  (params (OtherActor :type Actor%20Object%20Reference))
  (bind _teraccgda (Variables|Default|Getteraccgda))
  (bind _char_damage (Variables|Default|GetChar_Damage))
  (Utilities|Casting|CastToAmmoBase OtherActor)
  (bind _output_get (Variables|Default|Setbarrel_health (- (Variables|Default|Getbarrel_health) 25.0)))
  (if (<= _output_get 25.0)
    (Rendering|SetVisibility (Variables|Default|GetPointLight) true false)
    (Components|Activation|Activate (Variables|Default|Getfire) false)
    (Utilities|FlowControl|Delay 2.0)
    (Audio|PlaySound2D "/Game/StarterContent/Audio/Explosion_Cue.Explosion_Cue" 1.0 1.0 0.0 0 0)
    (Utilities|IsValid _char_damage
      (:Is%20Valid
        (Components|Sphere|SetSphereRadius _char_damage 1e+03 true)
        (Components|Sphere|SetSphereRadius (Variables|Default|Getbarrel_damage) 1e+03 true)
        (Components|DestroyComponent _char_damage))
      (:Is%20Not%20Valid
        _))
    (Class|RadialForceComponent|FireImpulse (Variables|Default|GetRadialForce))
    (Components|Activation|SetAutoActivate (Variables|Default|Getexp) false)
    (Utilities|IsValid _teraccgda
      (:Is%20Valid
        (Components|DestroyComponent _teraccgda)
        (Utilities|FlowControl|Delay 0.2)
        (Components|Activation|Deactivate (Variables|Default|Getfire))
        (Rendering|SetVisibility (Variables|Default|GetPointLight) false false)
        (Utilities|FlowControl|Delay 1.0)
        (Actor|DestroyActor)))))

(event EventTick
  (params (DeltaSeconds :type Float%20%28single-precision%29)))

(fn ConstructionScript)