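; BP_Inventory is a slot-based inventory that stores an item class and amount per slot.
; On BeginPlay in New Game mode it sizes the slot array to the configured slot count.
; It packs the slot count and slots into a save struct.
; Slot lookup by index reports whether a slot is empty and reads the item's details from its class defaults, so no item instance is needed.
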(event EventBeginPlay
  (switch Utilities|FlowControl|Switch|SwitchonE_InventoryStartMode (Variables|Default|GetStart%20Mode)
    (:NewEnumerator0
      (Utilities|Array|Resize (Variables|Default|GetSlots) (Variables|Default|GetAmound%20of%20Slots)))))

(fn ConstructionScript)

(fn GetSaveData
  (return (Utilities|Struct|MakeS_SaveInventoryInfo (Variables|Default|GetAmound%20of%20Slots) (Variables|Default|GetSlots))))

(fn GetSlotInfofromIndex
  (params (Index :type Integer))
  (bind _slots (Variables|Default|GetSlots))
  (bind _output (Utilities|Array|Get(acopy) _slots Index))
  (bind (_item _amount) (Utilities|Struct|BreakS_SlotSignature _output))
  ;[1 1 1] проверяем не пустой ли слот
  (if (Utilities|IsValidClass _item)
    (return false (Utilities|GetClassDefaults _item) _amount)
    (else
      (return true "" 0))))