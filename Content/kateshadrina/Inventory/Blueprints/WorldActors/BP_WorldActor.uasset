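; BP_WorldActor is a pickup for an inventory item placed in the world, with a floating name widget.
; On BeginPlay it reads its Item class defaults to set the mesh and fill WorldItem_WB with name, stackability and Amount.
; Each Tick it turns the widget toward the player's FollowCamera.
; The Pickup overlap toggles input; pressing F sets the cached MainCharacter's Pickup flag and destroys the actor, without passing item data.
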(event OnComponentBeginOverlap(pickup)
  (params (OverlappedComponent :type Primitive%20Component%20Object%20Reference) (OtherActor :type Actor%20Object%20Reference) (OtherComp :type Primitive%20Component%20Object%20Reference) (OtherBodyIndex :type Integer) (bFromSweep :type Boolean) (SweepResult :type Hit%20Result%20Structure%20%28by%20ref%29))
  (Input|EnableInput (Game|GetPlayerController 0))
  (bind _asmain_character (Utilities|Casting|CastToMainCharacter OtherActor)))

(event OnComponentEndOverlap(pickup)
  (params (OverlappedComponent :type Primitive%20Component%20Object%20Reference) (OtherActor :type Actor%20Object%20Reference) (OtherComp :type Primitive%20Component%20Object%20Reference) (OtherBodyIndex :type Integer))
  (Input|DisableInput (Game|GetPlayerController 0)))

(event EventBeginPlay
  ;[1 1 1] устанавливаем 3д меш и название итема
  (CallFunction|Initialize3DMesh)
  (CallFunction|InitialiseItemName))

(event EventTick
  (params (DeltaSeconds :type Float%20%28single-precision%29))
  ;[1 1 1] обновляем поворот виджета к камере персонажа
  (CallFunction|UpdateWidgetRotation))

(event Input|KeyboardEvents|F
  (params (Key :type Key%20Structure))
  (:Pressed
    (Variables|/Game/kateshadrina/Characters/MainCharacter.MainCharacter_C|Setpickup (stale OnComponentBeginOverlap(pickup) _asmain_character) true)
    (Actor|DestroyActor)))

(fn ConstructionScript)

(fn Initialize3DMesh
  (Components|StaticMesh|SetStaticMesh (Variables|Default|GetItemMesh) (.3dmesh (Utilities|GetClassDefaults (Variables|Default|GetItem)))))

(fn InitialiseItemName
  (bind _item (Variables|Default|GetItem))
  (bind _item_signature (Utilities|GetClassDefaults _item))
  (bind _asworld_item_wb (Utilities|Casting|CastToWorldItem_WB (UserInterface|GetUserWidgetObject (Variables|Default|GetWidget))))
  (Default|SetItemName _asworld_item_wb (.name _item_signature) (.stackablecanbestacked _item_signature) (Variables|Default|GetAmount)))

(fn UpdateWidgetRotation
  (Transformation|SetWorldRotation (Variables|Default|GetWidget) (Math|Rotator|FindLookatRotation (Transformation|GetWorldLocation (Variables|Default|GetWidget)) (Transformation|GetWorldLocation (Variables|/Game/kateshadrina/Characters/MainCharacter.MainCharacter_C|GetFollow%20camera (.AsMain%20Character (Utilities|Casting|CastToMainCharacter (Game|GetPlayerCharacter 0)))))) false false))